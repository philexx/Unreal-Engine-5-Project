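; BP_AICharacter is an AI-controlled character that reacts to perception and dies when its health runs out.
; Perception updates write each stimulus location to the LastSeenLocation Blackboard key, without filtering by sense or success.
; When the Health component reports zero or less, the mesh switches to ragdoll physics, the AI controller's brain logic stops and capsule collision is disabled.
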(event `self.ReceiveBeginPlay`)

(event `self.Health.OnHealthChanged`
  (params (HealthComp :type "HealthComponent Object Reference") (Health :type "Float (single-precision)") (HealthDelta :type "Float (single-precision)") (DamageType :type "DamageType Object Reference") (InstigatedBy :type "Controller Object Reference") (DamageCauser :type "Actor Object Reference"))
  (if (<= Health 0.0)
    (`PrimitiveComponent.SetSimulatePhysics` (`self.Mesh`) true)
    (`BrainComponent.StopLogic` (`AIController.BrainComponent` (`AIBlueprintHelperLibrary.GetAIController` self)) "Dead")
    (`PrimitiveComponent.SetCollisionEnabled` (`self.CapsuleComponent`) "NoCollision")))

(event `self.AIPerception.OnTargetPerceptionUpdated`
  (params (Actor :type "Actor Object Reference") (Stimulus :type "AIStimulus Structure"))
  (`BlackboardComponent.SetValueAsVector` (`AIBlueprintHelperLibrary.GetBlackboard` null) "LastSeenLocation" (`.StimulusLocation` (break `AIStimulus` Stimulus))))

(fn `UserConstructionScript`)