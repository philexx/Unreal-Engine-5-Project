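; Mission trigger actor that starts its UMission when a living SCharacterBase enters the overlap component E.
; Entry checks the HealthComponent's health, then either starts the mission or, if it is already completed, shows the Widget, which is hidden at BeginPlay and on exit.
; When the mission reports finished, one Niagara component switches to the completion effect and the second has its asset cleared.
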(event `self.ReceiveBeginPlay`
  (`SceneComponent.SetVisibility` (`self.Widget`) false false))

(event `self.e.OnComponentBeginOverlap`
  (params (OverlappedComponent :type "PrimitiveComponent Object Reference") (OtherActor :type "Actor Object Reference") (OtherComp :type "PrimitiveComponent Object Reference") (OtherBodyIndex :type Integer) (bFromSweep :type Boolean) (SweepResult :type "HitResult Structure (by ref)"))
  (bind _asscharacter_base (cast `SCharacterBase` OtherActor))
  (if (> (`HealthComponent.fHealth` (`self.GetComponentByClass` _asscharacter_base "/Script/Stealth.HealthComponent")) 0.0)
    (if (not (`UMissionComponent.bMissionCompleted` (`self.UMission`)))
      (`UMissionComponent.StartMission` (`self.UMission`))
      (else
        (`SceneComponent.SetVisibility` (`self.Widget`) true false)))))

(event `self.e.OnComponentEndOverlap`
  (params (OverlappedComponent :type "PrimitiveComponent Object Reference") (OtherActor :type "Actor Object Reference") (OtherComp :type "PrimitiveComponent Object Reference") (OtherBodyIndex :type Integer))
  (`SceneComponent.SetVisibility` (`self.Widget`) false false))

(event `self.UMission.OnMissionFinished`
  (params (Finished :type Boolean))
  (if Finished
    (`NiagaraComponent.SetAsset` (`self.Niagara`) "/Game/FX/NS_MissionStart_Complete.NS_MissionStart_Complete" true)
    (`NiagaraComponent.SetAsset` (`self.Niagara1`) null true)))

(fn `UserConstructionScript`)