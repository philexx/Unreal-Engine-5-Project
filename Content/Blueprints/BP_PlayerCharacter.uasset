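; Player character Blueprint that adds the HUD widgets and handles parkour moves, door kicks, takedowns and death.
; Movement events feed montage helpers that set Motion Warping targets and restore input on completion; takedowns instead slide the capsule to the AI's takedown point.
; The weapon wheel slows time, offsets the mouse to the current slot, then equips or unequips through WeaponInventory on release.
; Zero health triggers ragdoll, the death screen and a delayed level reload.
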(event `self.ReceiveBeginPlay`
  ;[0.2344 0.1825 0.1564] Begin Play
  (`|ExecutionSequence`
    (:`then_0`
      (bind _returnvalue (`|CreateWidget` "/Game/Widgets/InvetoryWidget/W_Inventory.W_Inventory_C"))
      (`UserWidget.AddToViewport` _returnvalue 0))
    (:`then_1`
      (bind _returnvalue_2 (`|CreateWidget` "/Game/Widgets/WBP_WeaponWheelHud.WBP_WeaponWheelHud_C"))
      (set `self.Weapon Wheel` _returnvalue_2)
      (`UserWidget.AddToViewport` _returnvalue_2 0))
    (:`then_2`
      (bind _returnvalue_3 (`|CreateWidget` "/Game/Widgets/WBP_Crosshair.WBP_Crosshair_C"))
      (`UserWidget.AddToViewport` _returnvalue_3 0))
    (:`then_3`
      (bind _returnvalue_4 (`|CreateWidget` "/Game/Widgets/WBP_UserInterface.WBP_UserInterface_C"))
      (`UserWidget.AddToViewport` _returnvalue_4 0))
    (:`then_4`
      (bind _returnvalue_5 (`|CreateWidget` "/Game/Widgets/WBP_DeadScreen.WBP_DeadScreen_C"))
      (set `self.Wasted_Widget` _returnvalue_5)
      (`UserWidget.AddToViewport` _returnvalue_5 0)
      (`Widget.SetVisibility` _returnvalue_5 "Hidden"))))

(event `InputAction|WeaponWheel`
  (params (Key :type "Key Structure"))
  (bind _returnvalue (`GameplayStatics.GetPlayerController` 0))
  (bind _weaponinventory (`self.WeaponInventory`))
  (bind _weapon_wheel (`self.Weapon Wheel`))
  (bind _fadeinout (`/Game/Widgets/WBP_WeaponWheelHud.FadeInOut` _weapon_wheel))
  (bind _w_weaponwheel (`/Game/Widgets/WBP_WeaponWheelHud.W_WeaponWheel` (`self.Weapon Wheel`)))
  (bind _currentslot (`WeaponWheel.CurrentSlot` (`/Game/Widgets/WBP_WeaponWheelHud.W_WeaponWheel` (`self.Weapon Wheel`))))
  ;[0.2077 1 0.3283] Open/Close WeaponWheel
  (:`Pressed`
    (set `WeaponWheel.IsOpen` true _w_weaponwheel)
    (`UserWidget.PlayAnimation` _weapon_wheel _fadeinout 0.0 1 "Reverse" 1.0 false)
    (`UserWidget.PlayAnimation` _weapon_wheel (`/Game/Widgets/WBP_WeaponWheelHud.Pulsing` _weapon_wheel) 0.0 0 "Forward" 1.0 false)
    (`GameplayStatics.SetGlobalTimeDilation` 0.08)
    (`WidgetBlueprintLibrary.SetInputMode_GameAndUIEx` _returnvalue (`self.Weapon Wheel`))
    (bind _returnvalue_2 (`self.CurrentSlotMousePositionOffset`))
    (bind _returnvalue_3 (`self.GetScreenCenter`))
    (`PlayerController.SetMouseLocation` _returnvalue (`KismetMathLibrary.FTrunc` (+ (`KismetMathLibrary.BreakVector2D` _returnvalue_2) (`KismetMathLibrary.BreakVector2D` _returnvalue_3))) (`KismetMathLibrary.FTrunc` (+ (`.Y` (`KismetMathLibrary.BreakVector2D` _returnvalue_2)) (`.Y` (`KismetMathLibrary.BreakVector2D` _returnvalue_3)))))
    (`GameplayStatics.PlaySound2D` "/Game/Widgets/Sounds/WhooshIn.WhooshIn" 0.6 1.0 0.5 null null)
    (bind _returnvalue_4 (`GameplayStatics.SpawnSound2D` "/Game/Widgets/Sounds/Heartbeat.Heartbeat" 0.6 1.0 0.0 null))
    (set `self.Heart Beat Ref` _returnvalue_4))
  (:`Released`
    (set `WeaponWheel.IsOpen` false _w_weaponwheel)
    (`GameplayStatics.SetGlobalTimeDilation` 1.0)
    (if (`KismetArrayLibrary.Array_IsEmpty` (`WeaponSlot.WeaponReference` _currentslot))
      (`WeaponInventory.UnequipWeapon` _weaponinventory)
      (else
        (`WeaponInventory.EquipWeapon` _weaponinventory (`WeaponSlot.CurrentWeapon` _currentslot))))
    (`UserWidget.PlayAnimation` _weapon_wheel _fadeinout 0.0 1 "Forward" 1.0 false)
    (`WidgetBlueprintLibrary.SetInputMode_GameOnly` _returnvalue)
    (`AudioComponent.Stop` (`self.Heart Beat Ref`))
    (`GameplayStatics.PlaySound2D` "/Game/Widgets/Sounds/WhooshOut.WhooshOut" 1.0 1.0 0.0 null null)))

(event `Key|G`
  (params (Key :type "Key Structure"))
  ;[1 0.1612 0.5548] Drop Weapon
  (:`Pressed`
    (`WeaponSlot.RemoveWeapon` (`WeaponWheel.CurrentSlot` (`/Game/Widgets/WBP_WeaponWheelHud.W_WeaponWheel` (`self.Weapon Wheel`))))))

(event `self.StartVault`
  (params (StartLocation :type "Vector Structure") (MidLocation :type "Vector Structure") (EndLocation :type "Vector Structure"))
  (bind _returnvalue (`self.K2_GetActorRotation`))
  (bind _charactermovement (`self.CharacterMovement`))
  (bind _motionwarping (`self.MotionWarping`))
  (bind (_returnvalue_location _returnvalue_rotation) (`KismetMathLibrary.BreakTransform` (`KismetMathLibrary.MakeTransform` MidLocation _returnvalue)))
  (bind (_returnvalue_location_2 _returnvalue_rotation_2) (`KismetMathLibrary.BreakTransform` (`KismetMathLibrary.MakeTransform` EndLocation _returnvalue)))
  ;[0.8338 0.2846 1] MotionWarp
  (if (!= StartLocation (0.0 0.0 0.0))
    (`CharacterMovementComponent.SetMovementMode` _charactermovement "MOVE_Flying" 0)
    (`self.DisableInput` (`GameplayStatics.GetPlayerController` 0))
    (`MotionWarpingComponent.AddOrUpdateWarpTarget` _motionwarping (make `MotionWarpingTarget` "StartMotionWarp" StartLocation _returnvalue))
    (`MotionWarpingComponent.AddOrUpdateWarpTarget` _motionwarping (make `MotionWarpingTarget` "LoopWarp" _returnvalue_location _returnvalue_rotation))
    (`MotionWarpingComponent.AddOrUpdateWarpTarget` _motionwarping (make `MotionWarpingTarget` "LandingWarp" _returnvalue_location_2 _returnvalue_rotation_2))
    (`|PlayMontage` (`self.Mesh`) "/Game/Character_Animation/AnimationMontages/VaultOverAnimMontage.VaultOverAnimMontage" 1.5
      (:`OnCompleted`
        (`CharacterMovementComponent.SetMovementMode` _charactermovement "MOVE_Walking" 0)
        (`self.EnableInput` (`GameplayStatics.GetPlayerController` 0) :!label _label)))))

(event `self.StartClimbLedge`
  (params (StartLocation :type "Vector Structure") (EndLocation :type "Vector Structure") (Rotation :type "Rotator Structure"))
  (bind _motionwarping (`self.MotionWarping`))
  ;[0.8338 0.2846 1] MotionWarp
  (`CharacterMovementComponent.SetMovementMode` (`self.CharacterMovement`) "MOVE_Flying" 0)
  (`self.DisableInput` (`GameplayStatics.GetPlayerController` 0))
  (`MotionWarpingComponent.AddOrUpdateWarpTarget` _motionwarping (make `MotionWarpingTarget` "StartLocationWarp" StartLocation Rotation))
  (`MotionWarpingComponent.AddOrUpdateWarpTarget` _motionwarping (make `MotionWarpingTarget` "EndLocationWarp" EndLocation Rotation))
  (`|PlayMontage` (`self.Mesh`) "/Game/Character_Animation/AnimationMontages/ClimbEdgeAnimMontage.ClimbEdgeAnimMontage"
    (:`OnCompleted`
      (`CharacterMovementComponent.SetMovementMode` (`self.CharacterMovement`) "MOVE_Walking" 0)
      (goto _label))))

(event `self.HangClimbLedgeMotionWarp`
  (params (StartLocation :type "Vector Structure") (EndLocation :type "Vector Structure") (Rotation :type "Rotator Structure"))
  ;[0.8338 0.2846 1] MotionWarp
  (`self.DisableInput` (`GameplayStatics.GetPlayerController` 0))
  (`MotionWarpingComponent.AddOrUpdateWarpTarget` (`self.MotionWarping`) (make `MotionWarpingTarget` "StartLocation" StartLocation Rotation))
  (`MotionWarpingComponent.AddOrUpdateWarpTarget` (`self.MotionWarping`) (make `MotionWarpingTarget` "EndLocation" EndLocation Rotation))
  (`|PlayMontage` (`self.Mesh`) "/Game/Traversal_Climb/Anim_MontageClimbTop.Anim_MontageClimbTop" 0.9
    (:`OnCompleted`
      (`CharacterMovementComponent.SetMovementMode` (`self.CharacterMovement`) "MOVE_Walking" 0)
      (goto _label))))

(event `self.JumpToNextMotionWarp`
  (params (MontageToPlay :type "AnimMontage Object Reference") (TargetLocation :type "Vector Structure") (TargetRotation :type "Rotator Structure"))
  ;[0.8338 0.2846 1] MotionWarp
  (`MotionWarpingComponent.AddOrUpdateWarpTarget` (`self.MotionWarping`) (make `MotionWarpingTarget` "EndLocation" TargetLocation TargetRotation))
  (`/Engine/EditorBlueprintResources/StandardMacros.IsValid` MontageToPlay
    (:`Is Valid`
      (`|PlayMontage` (`self.Mesh`) MontageToPlay
        (:`OnCompleted`
          (goto _label))))))

(event `self.KickInDoorWarp`
  (params (MontageToPlay :type "AnimMontage Object Reference") (TargetLocation :type "Vector Structure") (TargetRotation :type "Rotator Structure"))
  ;[0.8338 0.2846 1] MotionWarp
  (`self.DisableInput` (`GameplayStatics.GetPlayerController` 0))
  (`MotionWarpingComponent.AddOrUpdateWarpTarget` (`self.MotionWarping`) (make `MotionWarpingTarget` "TargetLocation" TargetLocation TargetRotation))
  (`/Engine/EditorBlueprintResources/StandardMacros.IsValid` MontageToPlay
    (:`Is Valid`
      (`|PlayMontage` (`self.Mesh`) MontageToPlay
        (:`OnCompleted`
          (goto _label))))))

(event `self.TakeDownMotionWarp`
  ;[0.8338 0.2846 1] MotionWarp
  (bind _asbp_aicharacter (cast `/Game/AI/BP_AICharacter` (`self.FocusedCharacter`)))
  (bind _takedown_location (`/Game/AI/BP_AICharacter.TakeDown Location` _asbp_aicharacter))
  (`KismetSystemLibrary.MoveComponentTo` (`self.CapsuleComponent`) (`SceneComponent.K2_GetComponentLocation` _takedown_location) (`SceneComponent.K2_GetComponentRotation` _takedown_location) true true)
  (`|PlayMontage` (`self.Mesh`) "/Game/Character_Animation/CombatAnimations/Paired_Knife_PlayerMontage.Paired_Knife_PlayerMontage"))

(event `Key|E`
  (params (Key :type "Key Structure"))
  (:`Pressed`
    (`ClimbingComponent.FindHangPoint` (`self.ClimbingComponent`))))

(event `self.UpdateWeaponSlotWidget`
  (params (Weapon :type "WeaponBase Object Reference"))
  ;[1 0.07269 0] c++ Update Weapon Wheel Slot
  (bind _returnvalue (`WeaponWheel.DetermineRightSlot` (`/Game/Widgets/WBP_WeaponWheelHud.W_WeaponWheel` (`self.Weapon Wheel`)) Weapon))
  (`WeaponSlot.AddWeapon` _returnvalue Weapon))

(event `self.HealthComponent.OnHealthChanged`
  (params (HealthComp :type "HealthComponent Object Reference") (Health :type "Float (single-precision)") (HealthDelta :type "Float (single-precision)") (DamageType :type "DamageType Object Reference") (InstigatedBy :type "Controller Object Reference") (DamageCauser :type "Actor Object Reference"))
  (if (<= Health 0.0)
    (`PrimitiveComponent.SetSimulatePhysics` (`self.Mesh`) true)
    (`self.DisableInput` (`GameplayStatics.GetPlayerController` 0))
    (`Widget.SetVisibility` (`self.Wasted_Widget`) "Visible")
    (`KismetSystemLibrary.Delay` 3.0)
    (`Widget.SetVisibility` (`self.Wasted_Widget`) "Hidden")
    (`GameplayStatics.OpenLevel` "Blockout")))

(event `self.ReceiveTick`
  (params (DeltaSeconds :type "Float (single-precision)")))

(fn `CurrentSlotMousePositionOffset`
  (returns (ReturnValue :type "Vector2D Structure"))
  (return (select `int` (- (`WeaponWheel.CurrentIndex` (`/Game/Widgets/WBP_WeaponWheelHud.W_WeaponWheel` (`self.Weapon Wheel`))) 1) :`0` (5.0 -15.0) :`1` (30.0 -5.0) :`2` (35.0 25.0) :`3` (-5.0 30.0) :`4` (-30.0 15.0) :`5` (-25.0 -30.0) :!type "Vector2D Structure")))

(fn `GetScreenCenter`
  (returns (ReturnValue :type "Vector2D Structure"))
  (return (- (/ (`WidgetLayoutLibrary.GetViewportSize`) (2.0 2.0)) (70.0 38.0))))

(fn `UserConstructionScript`)